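; Modular-mesh player character Blueprint that assembles a body and separate clothing and hair meshes in its Construction Script.
; Top, bottom, underwear, footwear and hair components follow the main Mesh's pose through Set Leader Pose Component.
; A dynamic skin material, created if not already valid, receives shoe and underwear mask textures, while fixed materials fill the eye, teeth and tongue slots.
; The Event Graph has no gameplay logic.
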(event `self.ReceiveBeginPlay`)

(fn `UserConstructionScript`
  (bind _skin_material (`self.Skin Material`))
  (bind _mesh (`self.Mesh`))
  (`|ExecutionSequence`
    (:`then_0`
      ;[1 1 1] Set leader pose
      (`SkinnedMeshComponent.SetLeaderPoseComponent` (`self.Top`) (`self.Mesh`) false false)
      (`SkinnedMeshComponent.SetLeaderPoseComponent` (`self.Bottom`) (`self.Mesh`) false false)
      (`SkinnedMeshComponent.SetLeaderPoseComponent` (`self.Underwear Bottom`) (`self.Mesh`) false false)
      (`SkinnedMeshComponent.SetLeaderPoseComponent` (`self.Shones`) (`self.Mesh`) false false)
      (`SkinnedMeshComponent.SetLeaderPoseComponent` (`self.Hair`) (`self.Mesh`) false false))
    (:`then_1`
      ;[1 1 1] Set skin material
      (`/Engine/EditorBlueprintResources/StandardMacros.IsValid` (`self.Skin Material`)
        (:`Is Valid`
          _)
        (:`Is Not Valid`
          (bind _returnvalue (`KismetMaterialLibrary.CreateDynamicMaterialInstance` "/Game/GR_Stylized_Female_01/Character/Materials/Skin/MT_Skin_Inst.MT_Skin_Inst"))
          (set `self.Skin Material` _returnvalue)))
      (`PrimitiveComponent.SetMaterial` (`self.Mesh`) 0 _skin_material)
      (`MaterialInstanceDynamic.SetTextureParameterValue` _skin_material "Feet Mask" "/Game/GR_Stylized_Female_01/Character/Textures/Shoe_01/shoes01_MASK.shoes01_MASK")
      (`MaterialInstanceDynamic.SetScalarParameterValue` _skin_material "Use Feet Mask" 1.0)
      (`MaterialInstanceDynamic.SetTextureParameterValue` _skin_material "Bottom Cloth Mask" "/Game/GR_Stylized_Female_01/Character/Textures/Underwear_01/underwear_bottom_MASK.underwear_bottom_MASK")
      (`MaterialInstanceDynamic.SetScalarParameterValue` _skin_material "Use Bottom Cloth Mask" 1.0)
      (`PrimitiveComponent.SetMaterial` _mesh 1 "/Game/GR_Stylized_Female_01/Character/Materials/Eyes/Materials/M_Sparrow_EyeRefractive_Inst2.M_Sparrow_EyeRefractive_Inst2")
      (`PrimitiveComponent.SetMaterial` _mesh 3 "/Game/GR_Stylized_Female_01/Character/Materials/Skin/MT_Tongue.MT_Tongue")
      (`PrimitiveComponent.SetMaterial` _mesh 2 "/Game/GR_Stylized_Female_01/Character/Materials/Skin/MT_Teeth.MT_Teeth")
      (`PrimitiveComponent.SetMaterial` _mesh 4 "/Game/GR_Stylized_Female_01/Character/Materials/Skin/MT_Tongue.MT_Tongue"))))