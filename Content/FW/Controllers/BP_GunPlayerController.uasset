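; BP_GunPlayerController is a player controller that relays HUD updates to the player's gun HUD widget.
; Its events set crosshair visibility and update main health, ammo bar, and per-slot health and color.
; Each event casts the result of GetGunHUD to WBP_HUD and forwards its values, doing nothing if the cast fails.
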(event `self.ShowCrosshair`
  (params (bShow :type Boolean))
  ;[1 1 1] HUD Update
  (bind _aswbp_hud (cast `/Game/FW/UI/WBP_HUD` (`self.GetGunHUD`)))
  (`/Game/FW/UI/WBP_HUD.SetCrosshairVisibility` _aswbp_hud bShow))

(event `self.UpdateMainHealthBar`
  (params (Health :type "Float (single-precision)") (MaxHealth :type "Float (single-precision)"))
  ;[1 1 1] HUD Update
  (bind _aswbp_hud (cast `/Game/FW/UI/WBP_HUD` (`self.GetGunHUD`)))
  (`/Game/FW/UI/WBP_HUD.Update Main Health` _aswbp_hud Health MaxHealth))

(event `self.UpdateAmmoBar`
  (params (percent :type "Float (single-precision)") (Color :type "LinearColor Structure"))
  ;[1 1 1] HUD Update
  (bind _aswbp_hud (cast `/Game/FW/UI/WBP_HUD` (`self.GetGunHUD`)))
  (`/Game/FW/UI/WBP_HUD.Update Ammo Bar` _aswbp_hud percent Color))

(event `self.UpdateSlotHealth`
  (params (slot :type Integer) (percent :type "Float (single-precision)"))
  ;[1 1 1] HUD Update
  (bind _aswbp_hud (cast `/Game/FW/UI/WBP_HUD` (`self.GetGunHUD`)))
  (`/Game/FW/UI/WBP_HUD.Update Slots Health` _aswbp_hud slot percent))

(event `self.UpdateSlotColor`
  (params (slot :type Integer) (Color :type "LinearColor Structure"))
  ;[1 1 1] HUD Update
  (bind _aswbp_hud (cast `/Game/FW/UI/WBP_HUD` (`self.GetGunHUD`)))
  (`/Game/FW/UI/WBP_HUD.Update Slots Color` _aswbp_hud slot Color))

(fn `UserConstructionScript`)